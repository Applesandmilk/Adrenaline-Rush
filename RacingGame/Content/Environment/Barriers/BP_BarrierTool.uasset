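; BP_BarrierTool is a level-building tool that lays a straight row of repeated barrier meshes from the actor's origin to an EndPoint.
; The construction script assigns MeshToSpawn and Scale to an instanced static mesh component, then fits as many whole Width segments as the scale-adjusted distance allows.
; Each instance is centered in its segment and rotated toward EndPoint.
; The event graph holds only disabled placeholder events.
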(fn `UserConstructionScript`
  (bind _width (`self.Width`))
  (bind _returnvalue (`KismetMathLibrary.FindLookAtRotation` (0.0 0.0 0.0) (`self.EndPoint`)))
  (`StaticMeshComponent.SetStaticMesh` (`self.InstancedStaticMesh`) (`self.MeshToSpawn`))
  (`SceneComponent.SetRelativeScale3D` (`self.InstancedStaticMesh`) (`self.Scale`))
  (for _index (range 1 (+ (`KismetMathLibrary.FFloor` (/ (`KismetMathLibrary.VSize` (/ (`self.EndPoint`) (`self.Scale`))) (`self.Width`))) 1))
    (`InstancedStaticMeshComponent.AddInstance` (`self.InstancedStaticMesh`) (`KismetMathLibrary.MakeTransform` (* (- (* _index _width) (/ _width 2.0)) (`KismetMathLibrary.GetForwardVector` _returnvalue)) _returnvalue) false)))